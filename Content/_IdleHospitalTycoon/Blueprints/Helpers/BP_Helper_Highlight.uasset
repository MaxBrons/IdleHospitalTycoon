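; Helper Blueprint that creates highlight copies of the meshes listed in ActorToHighlight, tinted with a configurable color.
; On BeginPlay it adds a collision-free static mesh component for each entry, copying that entry's mesh and relative transform.
; When SelectMaterial is valid, each copy gets a dynamic instance of it on every material slot, with the "Highlight Color" parameter set to HighlightColor.
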(event `self.ReceiveBeginPlay`
  (for _array_element (`self.Actor To Highlight`)
    (bind _returnvalue (`AddComponent|NODE_AddStaticMeshComponent-0` :`RelativeTransform` (`SceneComponent.GetRelativeTransform` _array_element)))
    (`StaticMeshComponent.SetStaticMesh` _returnvalue (`StaticMeshComponent.StaticMesh` _array_element))
    (`PrimitiveComponent.SetCollisionEnabled` _returnvalue "NoCollision")
    (bind _select_material (`self.Select Material`)
      (:`then`
        (bind _returnvalue_2 (`KismetMaterialLibrary.CreateDynamicMaterialInstance` _select_material))
        (for _index (range (`PrimitiveComponent.GetNumMaterials` _returnvalue))
          (`PrimitiveComponent.SetMaterial` _returnvalue _index _returnvalue_2)
          (`MaterialInstanceDynamic.SetVectorParameterValue` _returnvalue_2 "Highlight Color" (`self.Highlight Color`))))
      (:`else`))))

(fn `UserConstructionScript`)