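; Main menu pawn for the hospital tycoon game that handles click selection of world objects and 3D widgets.
; BeginPlay shows the mouse cursor and sets the WidgetInteraction source to match.
; Fire traces on Visibility, from the cursor in viewport UI mode or along the camera's forward vector otherwise.
; The hit actor's Comp_Select receives a select message, and a hit widget component's WB_Widget_Base gets SelectWidget.
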(event `self.ReceiveBeginPlay`
  (`self.Setup Mouse Interaction` true))

(event `InputAction|Fire` :paused true
  (params (Key :type "Key Structure"))
  (bind (_outhit _returnvalue) (`self.Get Trace Result For Objects`))
  (bind (_bblockinghit _binitialoverlap _time _distance _location _impactpoint _normal _impactnormal _physmat _hitactor _hitcomponent) (`GameplayStatics.BreakHitResult` _outhit))
  (bind _returnvalue_2 (`self.GetComponentByClass` _hitactor "/Game/_IdleHospitalTycoon/Blueprints/Components/Interaction/Comp_Select.Comp_Select_C"))
  ;[1 1 1] Component Selection
  (:`Pressed`
    (`|ExecutionSequence`
      (:`then_0`
        (if _returnvalue
          (`|ExecutionSequence`
            (:`then_0`
              (`/Engine/EditorBlueprintResources/StandardMacros.IsValid` _returnvalue_2
                (:`Is Valid`
                  (message `/Game/_IdleHospitalTycoon/Interfaces/I_Select.Select` _returnvalue_2 _location self _hitactor _hitcomponent))))
            (:`then_1`
              (bind _aswidget_component (cast `WidgetComponent` _hitcomponent))
              (bind _aswb_widget_base (cast `/Game/_IdleHospitalTycoon/Blueprints/Widgets/WB_Widget_Base` (`WidgetComponent.GetUserWidgetObject` _aswidget_component)))
              (`/Game/_IdleHospitalTycoon/Blueprints/Widgets/WB_Widget_Base.Select Widget` _aswb_widget_base))))))))

(fn `Get Trace Locations`
  (returns (`Trace Start` :type "Vector Structure") (`Trace End` :type "Vector Structure"))
  (bind _camera1 (`self.Camera1`))
  (bind _returnvalue (`SceneComponent.K2_GetComponentLocation` _camera1))
  (return _returnvalue (+ (* (`KismetMathLibrary.GetForwardVector` (`SceneComponent.K2_GetComponentRotation` _camera1)) 5000.0) _returnvalue)))

(fn `Get Trace Result For Objects`
  (returns (OutHit :type "HitResult Structure") (ReturnValue :type Boolean))
  (bind (_trace_start _trace_end) (`self.Get Trace Locations`))
  (bind (_hitresult _returnvalue) (`PlayerController.GetHitResultUnderCursorByChannel` (`GameplayStatics.GetPlayerController` 0) "TraceTypeQuery1" false))
  (if (`self.Viewport UI Mode Active`)
    (return _hitresult _returnvalue)
    (else
      (bind (_outhit _returnvalue_2) (`KismetSystemLibrary.LineTraceSingle` :`Start` _trace_start :`End` _trace_end :`TraceChannel` "TraceTypeQuery1" :`DrawDebugType` "ForDuration"))
      (return _outhit _returnvalue_2))))

(fn `Setup Mouse Interaction`
  (params (`Show Mouse Cursor` :type Boolean))
  (bind _output_get (set `PlayerController.bShowMouseCursor` `Show Mouse Cursor` (`GameplayStatics.GetPlayerController` 0)))
  (set `WidgetInteractionComponent.InteractionSource` (select `bool` _output_get :`false` "World" :`true` "Mouse" :!type "EWidgetInteractionSource Enum") (`self.WidgetInteraction`)))

(fn `UserConstructionScript`)