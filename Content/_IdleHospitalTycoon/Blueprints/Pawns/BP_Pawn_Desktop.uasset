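; Desktop player pawn for Idle Hospital Tycoon, handling flying camera movement, object selection, coins, pausing and the win screen.
; Traces from the camera, or under the cursor in UI mode, notify Comp_Select components and WB_Widget_Base widgets.
; Opening the HUD enables cursor mode and blocks mouse look; coin changes update the stats HUD, whose patient count triggers a retitled pause screen on winning.
; Tick feeds normalized pawn height into an audio parameter.
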(event `Key|Enter` :paused true
  (params (Key :type "Key Structure"))
  ;[1 1 1] Pause the game or quit the game
  (:`Pressed`
    (`/Engine/EditorBlueprintResources/StandardMacros.Gate` true :!label _label
      (:`Exit`
        (`KismetSystemLibrary.QuitGame` null "Quit")))))

(event `Key|Escape` :paused true
  (params (Key :type "Key Structure"))
  ;[1 1 1] Pause the game or quit the game
  (:`Pressed`
    (`self.Toggle Game Pause`)))

(event `Toggle Game Pause`
  ;[1 1 1] Pause the game or quit the game
  (bind _isa (`/Engine/EditorBlueprintResources/StandardMacros.FlipFlop`)
    (:`A`
      (`|ExecutionSequence`
        (:`then_0`
          (goto _label :!via `Open`))
        (:`then_1`
          _)))
    (:`B`
      (`|ExecutionSequence`
        (:`then_0`
          _)
        (:`then_1`
          (goto _label :!via `Close`)))))
  (`GameplayStatics.SetGamePaused` _isa)
  (bind _pause_screen_widget (`self.Pause Screen Widget`)
    (:`then`
      (`Widget.RemoveFromParent` _pause_screen_widget)
      (set `self.Pause Screen Widget` null))
    (:`else`
      (bind _returnvalue (`|CreateWidget` "/Game/_IdleHospitalTycoon/Blueprints/Widgets/HUD/Player/WB_PausedScreen.WB_PausedScreen_C" (`GameplayStatics.GetPlayerController` 0) (`self.Pause Screen Title`) (`self.Pause Screen Message`)))
      (bind _output_get (set `self.Pause Screen Widget` _returnvalue))
      (`UserWidget.AddToViewport` _output_get 10))))

(event `self.ReceiveBeginPlay`
  ;[1 1 1] Add the base HUD to player viewport
  (`self.AddControllerPitchInput` 10.0)
  (bind _returnvalue (`|CreateWidget` (`self.Player HUD Class To Spawn`) (`GameplayStatics.GetPlayerController` 0)))
  (bind _aswb_stats_hud (cast `/Game/_IdleHospitalTycoon/Blueprints/Widgets/HUD/Player/WB_StatsHUD` _returnvalue)
    (:`then`
      (bind _output_get (set `self.Player Stats HUD Widget` _aswb_stats_hud))
      (`UserWidget.AddToViewport` _output_get -1))
    (:`CastFailed`
      _))
  (bind _player_stats_hud_widget (`self.Player Stats HUD Widget`)
    (:`then`
      (`/Game/_IdleHospitalTycoon/Blueprints/Widgets/HUD/Player/WB_StatsHUD.Set Coins` _player_stats_hud_widget (`self.Coins`))
      (add `/Game/_IdleHospitalTycoon/Blueprints/Widgets/HUD/Player/WB_StatsHUD.On Stats Changed` _player_stats_hud_widget (delegate `Stats Changed`)))
    (:`else`
      _))
  (`AudioComponent.Play` (`self.Audio`) 0.0))

(event `Stats Changed`
  (params (Coins :type Integer) (`Helped Patients` :type Integer) (`Time Played` :type "Float (double-precision)"))
  ;[1 1 1] Add the base HUD to player viewport
  (if (>= `Helped Patients` (`self.Patient Amount To Help To Win`))
    (`self.Switch Pause Menu Info` (`self.Winning Title`) (`self.Winning Message`))))

(event `InputAction|Fire` :paused true
  (params (Key :type "Key Structure"))
  (bind (_outhit _returnvalue) (`self.Get Trace Result For Objects`))
  (bind (_bblockinghit _binitialoverlap _time _distance _location _impactpoint _normal _impactnormal _physmat _hitactor _hitcomponent) (`GameplayStatics.BreakHitResult` _outhit))
  (bind _returnvalue_2 (`self.GetComponentByClass` _hitactor "/Game/_IdleHospitalTycoon/Blueprints/Components/Interaction/Comp_Select.Comp_Select_C"))
  ;[1 1 1] Component Selection
  (:`Pressed`
    (`|ExecutionSequence`
      (:`then_0`
        (if _returnvalue
          (`|ExecutionSequence`
            (:`then_0`
              (`/Engine/EditorBlueprintResources/StandardMacros.IsValid` _returnvalue_2
                (:`Is Valid`
                  (message `/Game/_IdleHospitalTycoon/Interfaces/I_Select.Select` _returnvalue_2 _location self _hitactor _hitcomponent))))
            (:`then_1`
              (bind _aswidget_component (cast `WidgetComponent` _hitcomponent))
              (bind _aswb_widget_base (cast `/Game/_IdleHospitalTycoon/Blueprints/Widgets/WB_Widget_Base` (`WidgetComponent.GetUserWidgetObject` _aswidget_component)))
              (`/Game/_IdleHospitalTycoon/Blueprints/Widgets/WB_Widget_Base.Select Widget` _aswb_widget_base)))))
      (:`then_1`
        (`self.On Select Pressed` _outhit self)
        (set `self.Previous Hit Result` _outhit)))))

(event `InputAxis|MoveUp`
  (params (AxisValue :type "Float (single-precision)"))
  ;[1 1 1] Movement for moving up and down
  (if (`self.Input Blocked`)
    _
    (else
      _))
  (`self.AddMovementInput` (`SceneComponent.GetUpVector` (`self.CapsuleComponent`)) (* AxisValue (`self.Movement Speed`) (`GameplayStatics.GetWorldDeltaSeconds`))))

(event `Set Viewport UI Mode`
  (params (Active :type Boolean :default true))
  (bind _returnvalue (`GameplayStatics.GetPlayerController` 0))
  (bind (_sizex _sizey) (`PlayerController.GetViewportSize` _returnvalue))
  ;[1 1 1] Togle UI Mode
  (`self.Setup Mouse Interaction` Active)
  (bind _output_get (set `self.Viewport UI Mode Active` Active))
  (if _output_get
    (`WidgetBlueprintLibrary.SetInputMode_GameAndUIEx` _returnvalue null "LockAlways" false)
    (else
      (`WidgetBlueprintLibrary.SetInputMode_GameOnly` _returnvalue)))
  (`PlayerController.SetMouseLocation` _returnvalue (/ _sizex 2) (/ _sizey 2)))

(event `InputAxis|MoveForward`
  (params (AxisValue :type "Float (single-precision)"))
  ;[1 1 1] Movement for moving forward or backwards
  (if (`self.Input Blocked`)
    _
    (else
      _))
  (`self.AddMovementInput` (`SceneComponent.GetForwardVector` (`self.CapsuleComponent`)) (* AxisValue (`self.Movement Speed`) (`GameplayStatics.GetWorldDeltaSeconds`))))

(event `InputAction|Control`
  (params (Key :type "Key Structure"))
  (bind _charactermovement (`self.CharacterMovement`))
  (bind _movement_multiplier (`self.Movement Multiplier`))
  (bind _maxflyspeed (`CharacterMovementComponent.MaxFlySpeed` _charactermovement))
  ;[1 1 1] Increase Movement Speed
  (:`Pressed`
    (set `CharacterMovementComponent.MaxFlySpeed` (* _maxflyspeed _movement_multiplier) _charactermovement))
  (:`Released`
    (set `CharacterMovementComponent.MaxFlySpeed` (/ _maxflyspeed _movement_multiplier) _charactermovement)))

(event `Open HUD`
  (params (`Content Widget` :type "/Game/_IdleHospitalTycoon/Blueprints/Widgets/HUD/WB_HUD_Content Object Reference"))
  (bind _comp_widget (`self.Comp_Widget`))
  ;[1 1 1] Open and close the player HUD
  (bind _aswb_player_hud_base (cast `/Game/_IdleHospitalTycoon/Blueprints/Widgets/HUD/WB_PlayerHUD_Base` (`WidgetComponent.GetUserWidgetObject` _comp_widget)))
  (`/Game/_IdleHospitalTycoon/Blueprints/Widgets/HUD/WB_PlayerHUD_Base.Show HUD` _aswb_player_hud_base `Content Widget`)
  (`SceneComponent.SetVisibility` _comp_widget true false)
  (`self.Set Viewport UI Mode` true))

(event `InputAxis|MoveRight`
  (params (AxisValue :type "Float (single-precision)"))
  ;[1 1 1] Movement for moving right and left
  (if (`self.Input Blocked`)
    _
    (else
      _))
  (`self.AddMovementInput` (`SceneComponent.GetRightVector` (`self.CapsuleComponent`)) (* AxisValue (`self.Movement Speed`) (`GameplayStatics.GetWorldDeltaSeconds`))))

(event `Close HUD`
  ;[1 1 1] Open and close the player HUD
  (bind _aswb_player_hud_base (cast `/Game/_IdleHospitalTycoon/Blueprints/Widgets/HUD/WB_PlayerHUD_Base` (`WidgetComponent.GetUserWidgetObject` (`self.Comp_Widget`))))
  (`/Game/_IdleHospitalTycoon/Blueprints/Widgets/HUD/WB_PlayerHUD_Base.Hide HUD` _aswb_player_hud_base)
  (add `/Game/_IdleHospitalTycoon/Blueprints/Widgets/HUD/WB_PlayerHUD_Base.HUD Hidden` _aswb_player_hud_base (delegate `On HUD Hidde`)))

(event `On HUD Hidde`
  (params (`Hidden HUD Content` :type "/Game/_IdleHospitalTycoon/Blueprints/Widgets/HUD/WB_HUD_Content Object Reference") (`HUD Reference` :type "/Game/_IdleHospitalTycoon/Blueprints/Widgets/HUD/WB_PlayerHUD_Base Object Reference"))
  ;[1 1 1] Open and close the player HUD
  (remove `/Game/_IdleHospitalTycoon/Blueprints/Widgets/HUD/WB_PlayerHUD_Base.HUD Hidden` `HUD Reference` (delegate `On HUD Hidde`))
  (`SceneComponent.SetVisibility` (`self.Comp_Widget`) false false)
  (`self.Set Viewport UI Mode` false))

(event `InputAxis|Zoom`
  (params (AxisValue :type "Float (single-precision)"))
  ;[1 1 1] Movement for zooming in
)

(event `InputAxis|Turn`
  (params (AxisValue :type "Float (single-precision)"))
  (bind (_mouse_sensitivity_x _mouse_sensitivity_y) (`KismetMathLibrary.BreakVector2D` (`self.Mouse Sensitivity`)))
  ;[1 1 1] Handle rotation. Only rotate when the right mousebutton is pressed
  (if (not (`self.Input Blocked`))
    (`self.AddControllerYawInput` (* AxisValue _mouse_sensitivity_x (`GameplayStatics.GetWorldDeltaSeconds`)) :!label _label_2)))

(event `Add Coins`
  (params (Amount :type Integer))
  ;[1 1 1] Add or remove coins
  (set `self.Coins` (+ (`self.Coins`) Amount))
  (bind _player_stats_hud_widget (`self.Player Stats HUD Widget` :!label _label_3)
    (:`then`
      (`/Game/_IdleHospitalTycoon/Blueprints/Widgets/HUD/Player/WB_StatsHUD.Set Coins` _player_stats_hud_widget (`self.Coins`)))
    (:`else`)))

(event `InputAction|Select`
  (params (Key :type "Key Structure"))
  (bind (_mouse_sensitivity_x _mouse_sensitivity_y) (`KismetMathLibrary.BreakVector2D` (`self.Mouse Sensitivity`)))
  ;[1 1 1] Handle rotation. Only rotate when the right mousebutton is pressed
  (:`Pressed`
    (`|ExecutionSequence`
      (:`then_0`
        (`/Engine/EditorBlueprintResources/StandardMacros.Gate` true :!via `Open` :!label _label_4
          (:`Exit`
            (goto _label_2))))
      (:`then_1`
        (`/Engine/EditorBlueprintResources/StandardMacros.Gate` true :!via `Open` :!label _label_5
          (:`Exit`
            (`self.AddControllerPitchInput` (* (stale `InputAxis|LookUp` AxisValue) _mouse_sensitivity_y (`GameplayStatics.GetWorldDeltaSeconds`)) :!label _label_6))))))
  (:`Released`
    (`|ExecutionSequence`
      (:`then_0`
        (goto _label_4 :!via `Close`))
      (:`then_1`
        (goto _label_5 :!via `Close`)))))

(event `Remove Coins`
  (params (Amount :type Integer))
  ;[1 1 1] Add or remove coins
  (set `self.Coins` (- (`self.Coins`) Amount))
  (goto _label_3))

(event `InputAxis|LookUp`
  (params (AxisValue :type "Float (single-precision)"))
  ;[1 1 1] Handle rotation. Only rotate when the right mousebutton is pressed
  (if (not (`self.Input Blocked`))
    (goto _label_6)))

(event `self.ReceiveTick`
  (params (DeltaSeconds :type "Float (single-precision)"))
  (bind (_returnvalue_x _returnvalue_y _returnvalue_z) (`KismetMathLibrary.BreakVector` (`self.K2_GetActorLocation`)))
  ;[1 1 1] Audio mixing
  (bind _min_player_height_reference (`self.Min Player Height Reference`)
    (:`then`
      (bind _max_player_height_reference (`self.Max Player Height Reference`)
        (:`then`
          (bind (_returnvalue_x_2 _returnvalue_y_2 _returnvalue_z_2) (`KismetMathLibrary.BreakVector` (`self.K2_GetActorLocation` _min_player_height_reference)))
          (bind (_returnvalue_x_3 _returnvalue_y_3 _returnvalue_z_3) (`KismetMathLibrary.BreakVector` (`self.K2_GetActorLocation` _max_player_height_reference)))
          (`AudioComponent.SetFloatParameter` (`self.Audio`) "Player Air Height" (/ (`KismetMathLibrary.FClamp` (* (/ 100.0 (- _returnvalue_z_2 _returnvalue_z_3)) (- _returnvalue_z_2 _returnvalue_z)) 0.0 100.0) 100.0)))
        (:`else`)))
    (:`else`)))

(fn `Get Trace Locations`
  (returns (`Trace Start` :type "Vector Structure") (`Trace End` :type "Vector Structure"))
  (bind _returnvalue (`SceneComponent.K2_GetComponentLocation` (`self.Camera`)))
  (return _returnvalue (+ (* (`KismetMathLibrary.GetForwardVector` (`SceneComponent.K2_GetComponentRotation` (`self.Camera`))) 5000.0) _returnvalue)))

(fn `Get Trace Result For Objects`
  (returns (OutHit :type "HitResult Structure") (ReturnValue :type Boolean))
  (bind (_trace_start _trace_end) (`self.Get Trace Locations`))
  (bind (_hitresult _returnvalue) (`PlayerController.GetHitResultUnderCursorByChannel` (`GameplayStatics.GetPlayerController` 0) "TraceTypeQuery1" false))
  (if (`self.Viewport UI Mode Active`)
    (return _hitresult _returnvalue)
    (else
      (bind (_outhit _returnvalue_2) (`KismetSystemLibrary.LineTraceSingle` :`Start` _trace_start :`End` _trace_end :`TraceChannel` "TraceTypeQuery1" :`DrawDebugType` "ForDuration"))
      (return _outhit _returnvalue_2))))

(fn `Setup Mouse Interaction`
  (params (`Show Mouse Cursor` :type Boolean))
  (bind _output_get (set `PlayerController.bShowMouseCursor` `Show Mouse Cursor` (`GameplayStatics.GetPlayerController` 0)))
  (set `WidgetInteractionComponent.InteractionSource` (select `bool` _output_get :`false` "World" :`true` "Mouse" :!type "EWidgetInteractionSource Enum") (`self.WidgetInteraction`))
  (set `self.Input Blocked` _output_get))

(fn `Switch Pause Menu Info`
  (params (`Title Text` :type Text) (`Message Text` :type Text))
  (locals (Title :type Text) (Message :type Text))
  (set `local.Title` (`self.Pause Screen Title`))
  (set `local.Message` (`self.Pause Screen Message`))
  (set `self.Pause Screen Title` `Title Text`)
  (set `self.Pause Screen Message` `Message Text`)
  (`self.Toggle Game Pause`)
  (set `self.Pause Screen Title` (`local.Title`))
  (set `self.Pause Screen Message` (`local.Message`)))

(fn `UserConstructionScript`
  (`parent.UserConstructionScript`))