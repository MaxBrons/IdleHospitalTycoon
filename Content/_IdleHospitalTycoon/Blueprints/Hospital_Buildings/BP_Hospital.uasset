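; BP_Hospital is a selectable, purchasable hospital building for an idle tycoon game.
; BeginPlay creates unpurchased and purchased HUD widgets plus a first doctor, and selection opens the widget matching the hospital state.
; Widget events drive buying, which deducts pawn coins, switches state and updates highlight color, and adding doctors.
; Each doctor widget gets a spawned BP_Doctor actor linked to the hospital.
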(event `self.ReceiveBeginPlay`
  (bind (_unpurchased_content_titlename _unpurchased_content_contenttext _unpurchased_content_buttontext _unpurchased_content_buttonbackgroundcolor) (break `/Game/_IdleHospitalTycoon/Structs/S_Hospital_Content_Unpurchased` (`self.Unpurchased Content`)))
  (bind (_purchased_content_title _purchased_content_buttontext _purchased_content_buttonbackgroundcolor) (break `/Game/_IdleHospitalTycoon/Structs/S_Hospital_Content_Purchased` (`self.Purchased Content`)))
  ;[1 1 1] Create the widgets on start
  (bind _returnvalue (`|CreateWidget` "/Game/_IdleHospitalTycoon/Blueprints/Widgets/HUD/Hospital/WB_HUD_Content_Unpurchased.WB_HUD_Content_Unpurchased_C" null _unpurchased_content_titlename _unpurchased_content_contenttext _unpurchased_content_buttontext _unpurchased_content_buttonbackgroundcolor))
  (set `self.Unpurchased Widget` _returnvalue)
  (bind _returnvalue_2 (`|CreateWidget` "/Game/_IdleHospitalTycoon/Blueprints/Widgets/HUD/Hospital/WB_HUD_Content_Purchased.WB_HUD_Content_Purchased_C" null _purchased_content_title _purchased_content_buttontext _purchased_content_buttonbackgroundcolor))
  (set `self.Purchased Widget` _returnvalue_2)
  (`/Game/_IdleHospitalTycoon/Blueprints/Widgets/HUD/Hospital/WB_HUD_Content_Purchased.Add Doctor` _returnvalue_2 1 0.0 (struct :`G` 0.483937 :`B` 1.0 :`A` 1.0))
  (`self.Add Doctor` (`|GetArrayItem` (`/Game/_IdleHospitalTycoon/Blueprints/Widgets/HUD/Hospital/WB_HUD_Content_Purchased.Doctors` _returnvalue_2)))
  (set `self.Normal Highlight Color` (`/Game/_IdleHospitalTycoon/Blueprints/Components/Interaction/Comp_Highlight.Highlight Color` (`self.Comp_Highlight`)))
  (`self.Update Highlight Color`))

(event `Widget Functionality`
  (params (`Widget Reference` :type "/Game/_IdleHospitalTycoon/Blueprints/Widgets/WB_Widget_Base Object Reference") (Command :type Name) (`Object Reference` :type "Object Object Reference") (`Class Reference` :type "Object Class Reference"))
  (bind _purchase_price (`self.Purchase Price`))
  ;[1 1 1] Handle HUD opening, closing and functionality
  (switch `name` Command
    (:`Purchase`
      (bind _asbp_pawn_desktop (cast `/Game/_IdleHospitalTycoon/Blueprints/Pawns/BP_Pawn_Desktop` (`GameplayStatics.GetPlayerPawn` 0)))
      (if (>= (- (`/Game/_IdleHospitalTycoon/Blueprints/Pawns/BP_Pawn_Desktop.Coins` _asbp_pawn_desktop) _purchase_price) 0)
        (`/Game/_IdleHospitalTycoon/Blueprints/Pawns/BP_Pawn_Desktop.Remove Coins` _asbp_pawn_desktop _purchase_price)
        (`self.Update Hospital State` "NewEnumerator1")
        (`self.Update Highlight Color`)
        (`self.BndEvt__BP_Hospital_Comp_Select_K2Node_ComponentBoundEvent_1_Active State Changed__DelegateSignature` false (stale `self.Comp_Select.Active State Changed` `Pawn Reference`))))))

(event `self.Comp_Select.Active State Changed`
  (params (`Active State` :type Boolean) (`Pawn Reference` :type "/Game/_IdleHospitalTycoon/Blueprints/Pawns/BP_Pawn_Base Object Reference"))
  ;[1 1 1] Handle HUD opening, closing and functionality
  (bind _asbp_pawn_desktop (cast `/Game/_IdleHospitalTycoon/Blueprints/Pawns/BP_Pawn_Desktop` `Pawn Reference`))
  (switch `/Game/_IdleHospitalTycoon/Enums/E_HospitalState` (`self.Hospital State`)
    (:`NewEnumerator0`
      (bind _unpurchased_widget (`self.Unpurchased Widget`)
        (:`then`
          (`/Game/_IdleHospitalTycoon/Blueprints/Pawns/BP_Pawn_Desktop.Open HUD` _asbp_pawn_desktop _unpurchased_widget)
          (`/Engine/EditorBlueprintResources/StandardMacros.DoOnce` false
            (:`Completed`
              (add `/Game/_IdleHospitalTycoon/Blueprints/Widgets/WB_Widget_Base.Widget Functionality Event` _unpurchased_widget (delegate `Widget Functionality`)))))
        (:`else`)))
    (:`NewEnumerator1`
      (bind _purchased_widget (`self.Purchased Widget`)
        (:`then`
          (`/Game/_IdleHospitalTycoon/Blueprints/Pawns/BP_Pawn_Desktop.Open HUD` _asbp_pawn_desktop _purchased_widget)
          (add `/Game/_IdleHospitalTycoon/Blueprints/Widgets/WB_Widget_Base.Widget Functionality Event` _purchased_widget (delegate `Widget Functionality Event_Event_0`))
          (bind _unpurchased_widget_2 (`self.Unpurchased Widget`)
            (:`then`
              (remove `/Game/_IdleHospitalTycoon/Blueprints/Widgets/WB_Widget_Base.Widget Functionality Event` _unpurchased_widget_2 (delegate `Widget Functionality`)))
            (:`else`)))
        (:`else`)))))

(event `Update Hospital State`
  (params (`New State` :type "/Game/_IdleHospitalTycoon/Enums/E_HospitalState Enum" :default "NewEnumerator0"))
  ;[1 1 1] Set a new state
  (set `self.Hospital State` `New State`))

(event `Widget Functionality Event_Event_0`
  (params (`Widget Reference` :type "/Game/_IdleHospitalTycoon/Blueprints/Widgets/WB_Widget_Base Object Reference") (Command :type Name) (`Object Reference` :type "Object Object Reference") (`Class Reference` :type "Object Class Reference"))
  ;[1 1 1] Add doctor when add button is pressed
  (switch `name` Command
    (:`Purchased Doctor`
      (bind _aswb_doctor (cast `/Game/_IdleHospitalTycoon/Blueprints/Widgets/HUD/Hospital/Doctors/WB_Doctor` `Object Reference`))
      (`self.Add Doctor` _aswb_doctor))))

(event `Update Highlight Color`
  ;[1 1 1] Set Highlight Color
  (set `/Game/_IdleHospitalTycoon/Blueprints/Components/Interaction/Comp_Highlight.Highlight Color` (select `/Game/_IdleHospitalTycoon/Enums/E_HospitalState` (`self.Hospital State`) :`NewEnumerator0` (`self.Closed Highlight Color`) :`NewEnumerator1` (`self.Normal Highlight Color`)) (`self.Comp_Highlight`)))

(fn `Add Doctor`
  (params (`Doctor Widget` :type "/Game/_IdleHospitalTycoon/Blueprints/Widgets/HUD/Hospital/Doctors/WB_Doctor Object Reference"))
  (returns (`Spawned Doctor` :type "/Game/_IdleHospitalTycoon/Blueprints/Doctors/BP_Doctor Object Reference"))
  (bind _returnvalue (`|SpawnActorFromClass` "/Game/_IdleHospitalTycoon/Blueprints/Doctors/BP_Doctor.BP_Doctor_C" (`self.GetTransform`) "Undefined" "OverrideRootScale" null self 1 `Doctor Widget` 50 null))
  (`KismetArrayLibrary.Array_AddUnique` (`self.Doctors`) _returnvalue)
  (return _returnvalue))

(fn `UserConstructionScript`)